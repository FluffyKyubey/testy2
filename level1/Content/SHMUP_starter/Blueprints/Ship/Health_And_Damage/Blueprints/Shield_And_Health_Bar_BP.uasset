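; World-space health and shield bar actor that turns its arrow toward the player camera each Tick.
; Construction creates dynamic materials for both bars, whose "Health" parameter Tick drives, optionally smoothed with FInterpToConstant.
; Each bar can auto-read an element of the parent actor's Health_BP component arrays; index -1 uses its own variables.
; Optional current/max text hides at zero, and the shield display can switch off when health is zero.
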(event EventTick
  (params (DeltaSeconds :type Float%20%28single-precision%29))
  (bind _returnvalue (Game|GetPlayerController 0))
  (bind _returnvalue_2 (Actor|GetParentActor))
  (bind _returnvalue_3 (Actor|GetParentActor))
  (bind _auto_update_shield_from_element (Variables|Default|GetAuto%20Update%20Shield%20From%20Element))
  (bind _auto_update_health_from_element (Variables|Default|GetAuto%20Update%20Health%20From%20Element))
  (bind _health_text (Variables|Default|GetHealth_Text))
  (bind _shield_text (Variables|Default|GetShield%20Text))
  (bind _returnvalue_4 (Actor|GetComponentbyClass _returnvalue_2 "/Game/SHMUP_starter/Blueprints/Ship/Health_And_Damage/Blueprints/Health_BP.Health_BP_C"))
  (bind _returnvalue_5 (Actor|GetComponentbyClass _returnvalue_3 "/Game/SHMUP_starter/Blueprints/Ship/Health_And_Damage/Blueprints/Health_BP.Health_BP_C"))
  (bind _max_health (Variables|/Game/SHMUP_starter/Blueprints/Ship/Health_And_Damage/Blueprints/Health_BP.Health_BP_C|GetMax%20Health _returnvalue_5))
  (bind _current_health (Variables|/Game/SHMUP_starter/Blueprints/Ship/Health_And_Damage/Blueprints/Health_BP.Health_BP_C|GetCurrent%20Health _returnvalue_5))
  (bind _max_health_2 (Variables|/Game/SHMUP_starter/Blueprints/Ship/Health_And_Damage/Blueprints/Health_BP.Health_BP_C|GetMax%20Health _returnvalue_4))
  (bind _current_health_2 (Variables|/Game/SHMUP_starter/Blueprints/Ship/Health_And_Damage/Blueprints/Health_BP.Health_BP_C|GetCurrent%20Health _returnvalue_4))
  (bind _output (Utilities|Array|Get(acopy) _max_health _auto_update_shield_from_element))
  (bind _output_2 (Utilities|Array|Get(acopy) _current_health _auto_update_shield_from_element))
  (bind _output_3 (Utilities|Array|Get(acopy) _current_health_2 _auto_update_health_from_element))
  (bind _output_4 (Utilities|Array|Get(acopy) _max_health_2 _auto_update_health_from_element))
  (Utilities|FlowControl|Sequence
    (:then_0
      ;[1 1 1] Find if auto updating from Health_BP component
      (if (== (Variables|Default|GetAuto%20Update%20Health%20From%20Element) -1)
        _
        (else
          ;[1 1 1] Get values from Health BP component
          (Utilities|IsValid _returnvalue_2
            (:Is%20Valid
              (Variables|Default|SetCurrent%20Health%20Value _output_3)
              (Variables|Default|SetMax%20Health%20Value _output_4)
              (Variables|Default|SetHealth%20%25%20Value (* (/ _output_3 _output_4) 1e+02))))))
      ;[1 1 1] Set world rotation to point towards player camera
      (Utilities|IsValid _returnvalue
        (:Is%20Valid
          (Transformation|SetWorldRotation (Variables|Default|GetArrow) (Math|Rotator|FindLookatRotation (Transformation|GetWorldLocation (Variables|Default|GetArrow)) (Camera|GetCameraLocation (Variables|/Script/Engine.PlayerController|GetPlayerCameraManager _returnvalue))) false false))
        (:Is%20Not%20Valid
          _))
      ;[1 1 1] Check if updating with a delay
      (if (== (Variables|Default|GetVisual%20Delay%20Interp%20Speed) 0.0)
        ;[1 1 1] Update health value on material
        (Rendering|Material|SetScalarParameterValue (Variables|Default|GetHealth%20Bar%20Mat) "Health" (* (Variables|Default|GetHealth%20%25%20Value) 0.01) :!class /Script/Engine.MaterialInstanceDynamic)
        (else
          ;[1 1 1] Find Visual Value If Delaying Updates
          (Variables|Default|SetCurrent%20Health%20Value%20Visual (Math|Interpolation|FInterptoConstant (Variables|Default|GetCurrent%20Health%20Value%20Visual) (Variables|Default|GetCurrent%20Health%20Value) (Utilities|Time|GetWorldDeltaSeconds) (Variables|Default|GetVisual%20Delay%20Interp%20Speed)))
          ;[1 1 1] Update health value on material
          (Rendering|Material|SetScalarParameterValue (Variables|Default|GetHealth%20Bar%20Mat) "Health" (/ (Variables|Default|GetCurrent%20Health%20Value%20Visual) (Variables|Default|GetMax%20Health%20Value)) :!class /Script/Engine.MaterialInstanceDynamic)))
      ;[1 1 1] Update text value
      (if (Variables|Default|GetUse%20Text)
        (if (== (Variables|Default|GetHealth%20%25%20Value) 0.0)
          (Rendering|SetVisibility _health_text false false :!label _label)
          (else
            (Rendering|SetVisibility _health_text true false)
            (Rendering|Components|TextRender|SetText _health_text (Utilities|Text|FormatText "{A}/{B}" (Variables|Default|GetCurrent%20Health%20Value) (Variables|Default|GetMax%20Health%20Value)))))
        (else
          (goto _label))))
    (:then_1
      (if (Variables|Default|GetShield%20Bar%20Disabled%20On%20Health%20Bar%200)
        (if (== (Variables|Default|GetHealth%20%25%20Value) 0.0)
          (Rendering|Material|SetScalarParameterValue (Variables|Default|GetShield%20Bar%20Mat) "Health" 0.0 :!class /Script/Engine.MaterialInstanceDynamic)
          (Rendering|SetVisibility (Variables|Default|GetShield%20Text) false false)
          (else
            ;[1 1 1] Find if auto updating from Health_BP component
            (if (== (Variables|Default|GetAuto%20Update%20Shield%20From%20Element) -1) :!label _label_2
              _
              (else
                ;[1 1 1] Get values from Health BP component
                (Utilities|IsValid _returnvalue_3
                  (:Is%20Valid
                    (Variables|Default|SetCurrent%20Health%20Value%20%28Shield%29 _output_2)
                    (Variables|Default|SetMax%20Health%20Value%20%28Shield%29 _output)
                    (Variables|Default|SetShield%20%25%20Value (* (/ _output_2 _output) 1e+02))))))
            ;[1 1 1] Check if updating with a delay
            (if (== (Variables|Default|GetVisual%20Delay%20Interp%20Speed%20%28Shield%29) 0.0)
              ;[1 1 1] Update health value on material
              (Rendering|Material|SetScalarParameterValue (Variables|Default|GetShield%20Bar%20Mat) "Health" (* (Variables|Default|GetShield%20%25%20Value) 0.01) :!class /Script/Engine.MaterialInstanceDynamic)
              (else
                ;[1 1 1] Find Visual Value If Delaying Updates
                (Variables|Default|SetCurrent%20Health%20Value%20Visual%20%28Shield%29 (Math|Interpolation|FInterptoConstant (Variables|Default|GetCurrent%20Health%20Value%20Visual%20%28Shield%29) (Variables|Default|GetCurrent%20Health%20Value%20%28Shield%29) (Utilities|Time|GetWorldDeltaSeconds) (Variables|Default|GetVisual%20Delay%20Interp%20Speed%20%28Shield%29)))
                ;[1 1 1] Update health value on material
                (Rendering|Material|SetScalarParameterValue (Variables|Default|GetShield%20Bar%20Mat) "Health" (/ (Variables|Default|GetCurrent%20Health%20Value%20Visual%20%28Shield%29) (Variables|Default|GetMax%20Health%20Value%20%28Shield%29)) :!class /Script/Engine.MaterialInstanceDynamic)))
            ;[1 1 1] Update text value
            (if (Variables|Default|GetUse%20Text)
              (if (== (Variables|Default|GetShield%20%25%20Value) 0.0)
                (Rendering|SetVisibility _shield_text false false :!label _label_3)
                (else
                  (Rendering|SetVisibility _shield_text true false)
                  (Rendering|Components|TextRender|SetText _shield_text (Utilities|Text|FormatText "{A}/{B}" (Variables|Default|GetCurrent%20Health%20Value%20%28Shield%29) (Variables|Default|GetMax%20Health%20Value%20%28Shield%29)))))
              (else
                (goto _label_3)))))
        (else
          (goto _label_2))))))

(fn ConstructionScript
  (bind _health_text (Variables|Default|GetHealth_Text))
  ;[1 1 1] Create a dynamic material for the health bars
  (bind _returnvalue (Rendering|Material|CreateDynamicMaterialInstance (Variables|Default|GetHealth%20Bar) 0 0 "None" :!class /Script/Engine.PrimitiveComponent))
  (Variables|Default|SetHealth%20Bar%20Mat _returnvalue)
  (bind _returnvalue_2 (Rendering|Material|CreateDynamicMaterialInstance (Variables|Default|GetShield%20Bar) 0 0 "None" :!class /Script/Engine.PrimitiveComponent))
  (Variables|Default|SetShield%20Bar%20Mat _returnvalue_2)
  ;[1 1 1] Set initial text visibility
  (if (Variables|Default|GetUse%20Text)
    (Rendering|SetVisibility _health_text true false)
    (Rendering|Components|TextRender|SetText (Variables|Default|GetHealth_Text) (Utilities|Text|FormatText "{A}/{B}" (Variables|Default|GetCurrent%20Health%20Value) (Variables|Default|GetMax%20Health%20Value)))
    (Rendering|Components|TextRender|SetText (Variables|Default|GetShield%20Text) (Utilities|Text|FormatText "{A}/{B}" (Variables|Default|GetCurrent%20Health%20Value%20%28Shield%29) (Variables|Default|GetMax%20Health%20Value%20%28Shield%29)))
    ;[1 1 1] Current Health Value Update
    (Variables|Default|SetCurrent%20Health%20Value%20Visual%20%28Shield%29 (Variables|Default|GetCurrent%20Health%20Value%20%28Shield%29))
    (Variables|Default|SetCurrent%20Health%20Value%20Visual (Variables|Default|GetCurrent%20Health%20Value))
    (else
      (Rendering|SetVisibility _health_text false false))))