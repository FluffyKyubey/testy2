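; Demo shielded target that shows how an actor receives damage updates for a specific health element, here the head shield.
; DamageActor forwards damage, modifiers and hit component/bone to the Health component and returns its result, omitting causer and instigator.
; HealthChangeUpdate filters for the shield's index and prints damage dealt or power restored.
; Damage messages linger, while restore messages last two frames' time.
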(event EventBeginPlay)

(event Collision|EventActorBeginOverlap
  (params (OtherActor :type Actor%20Object%20Reference)))

(event EventHealthChangeUpdate
  (params (Index :type Integer) (Damage%20Taken :type Float%20%28single-precision%29) (Regen :type Boolean))
  (bind _returnvalue (>= Damage%20Taken 0.0))
  (bind _returnvalue_2 (Math|Conversions|ToFloat(Boolean) _returnvalue))
  ;[1 1 1] An example of gettign anupdate on any damage this actor receives to a given health element. In this case the head shield.
  (if (== Index 2)
    (Development|PrintText (Utilities|Text|FormatText "{A} {B}" (Math|Float|Lerp (* Damage%20Taken -1.0) Damage%20Taken _returnvalue_2) (select _returnvalue "Damage dealt to shield" "Power restored in shield")) true false "(R=0.000000,G=0.964972,B=1.000000,A=1.000000)" (Math|Float|Lerp (* (Utilities|Time|GetWorldDeltaSeconds) 2.0) 5.0 _returnvalue_2))))

(event EventTick
  (params (DeltaSeconds :type Float%20%28single-precision%29)))

(fn ConstructionScript)

(fn DamageActor
  (params (Damage%20Value :type Float%20%28single-precision%29) (Damage%20Modifiers :type Array%20of%20Strings) (Damaged%20Caused%20By :type Actor%20Object%20Reference) (Instigator :type Controller%20Object%20Reference) (Hit%20Component :type Actor%20Component%20Object%20Reference) (Hit%20Bone :type Name :default "None") (Damage%20All%20Parts :type Boolean))
  (bind (_damage_taken _relevant_modifiers) (Default|DamageActor (Variables|Default|GetHealth) Damage%20Value Damage%20Modifiers 0 0 Hit%20Component Hit%20Bone Damage%20All%20Parts))
  (return _damage_taken _relevant_modifiers))