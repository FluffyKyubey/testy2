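; Demo target actor for the SHMUP starter's health and damage system, made of five cubes that can be destroyed individually.
; DamageActor forwards hits to the Health component and returns the damage taken and relevant modifiers.
; Health change events print the damage per cube.
; Depletion calls ServerUpdateDeath, which uses a MultiGate as an index switch to destroy the matching cube, then resets it.
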(event Custom|Server%20Update%20Death
  (params (StartIndex :type Integer))
  (Utilities|FlowControl|Sequence
    (:then_0
      (Utilities|FlowControl|MultiGate false false StartIndex :!label _label
        (:Out%200
          (Components|DestroyComponent (Variables|Default|GetA)))
        (:Out%201
          (Components|DestroyComponent (Variables|Default|GetB)))
        (:Out%202
          (Components|DestroyComponent (Variables|Default|GetC)))
        (:Out%203
          (Components|DestroyComponent (Variables|Default|GetD)))
        (:Out%204
          (Components|DestroyComponent (Variables|Default|GetTop)))))
    (:then_1
      (goto _label Reset))))

(event EventBeginPlay)

(event Collision|EventActorBeginOverlap
  (params (OtherActor :type Actor%20Object%20Reference)))

(event EventHealthChangeUpdate
  (params (Index :type Integer) (Damage%20Taken :type Float%20%28single-precision%29) (Regen :type Boolean))
  ;[1 1 1] An example of gettign anupdate on any damage this actor receives to a given health element.
  (Development|PrintText (Utilities|Text|FormatText "{A} Damage dealt to {B}." Damage%20Taken (Utilities|Select :Index Index :Option%200 "A cube" :Option%201 "B cube" :Option%202 "C cube" :Option%203 "D cube" :Option%204 "Top cube")) true false "(R=1.000000,G=0.360092,B=0.000000,A=1.000000)" 5.0))

(event EventHealthDepleted
  (params (Health%20Element :type Integer) (Caused%20By%20Actor :type Actor%20Object%20Reference) (Instigator :type Controller%20Object%20Reference))
  (CallFunction|ServerUpdateDeath Health%20Element))

(event EventTick
  (params (DeltaSeconds :type Float%20%28single-precision%29)))

(fn ConstructionScript)

(fn DamageActor
  (params (Damage%20Value :type Float%20%28single-precision%29) (Damage%20Modifiers :type Array%20of%20Strings) (Damaged%20Caused%20By :type Actor%20Object%20Reference) (Instigator :type Controller%20Object%20Reference) (Hit%20Component :type Actor%20Component%20Object%20Reference) (Hit%20Bone :type Name :default "None") (Damage%20All%20Parts :type Boolean))
  (bind (_damage_taken _relevant_modifiers) (Default|DamageActor (Variables|Default|GetHealth) Damage%20Value Damage%20Modifiers Damaged%20Caused%20By Instigator Hit%20Component Hit%20Bone Damage%20All%20Parts))
  (return _damage_taken _relevant_modifiers))