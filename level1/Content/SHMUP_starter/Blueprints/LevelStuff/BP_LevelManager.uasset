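; Level manager for a shoot 'em up, scripting a timed sequence of enemy waves, asteroids, drop ships, level pieces and a robot mini-boss.
; It registers with BP_Hero, then runs StartPhase, whose robot receives a manager reference to trigger PhaseUp on death.
; PhaseUp steps through delay-timed phases, finally setting the hero's LevelMod1.
; Wave macros respawn themselves through SpawnEnemy until the shared Done flag breaks the loop.
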(event Custom|SpawnLevelObject
  (params (LevelPart :type Integer))
  ;[1 1 1] Spawning
  ;;[1 1 1] Spawn level objects
  (switch int LevelPart
    (:1
      (Game|SpawnActorfromClass "/Game/SHMUP_starter/Blueprints/LevelStuff/SampleLevel/BP_LevelTest_TopPart1.BP_LevelTest_TopPart1_C" (Math|Transform|MakeTransform "0,3500.000000,800.000000" "0, 0, 0" "1,1,1") "Undefined" 0 0)
      (Utilities|FlowControl|Delay 1e+01)
      (Game|SpawnActorfromClass "/Game/SHMUP_starter/Blueprints/LevelStuff/SampleLevel/BG_LevelTest_BottomPart1.BG_LevelTest_BottomPart1_C" (Math|Transform|MakeTransform "0,3500.000000,-600.000000" "0, 0, 0" "1,1,1") "Undefined" 0 0))
    (:2
      (Game|SpawnActorfromClass "/Game/SHMUP_starter/Blueprints/LevelStuff/SampleLevel/BP_LevelTest_BGPart1.BP_LevelTest_BGPart1_C" (Math|Transform|MakeTransform "2000.000000,15000.000000,0.000000" "0, 0, 0" "1,1,1") "Undefined" 0 0)
      (Utilities|FlowControl|Delay 5.0)
      (Game|SpawnActorfromClass "/Game/SHMUP_starter/Blueprints/LevelStuff/SampleLevel/BP_LevelTest_FGPart1.BP_LevelTest_FGPart1_C" (Math|Transform|MakeTransform "0,3500.000000,-600.000000" "0, 0, 0" "1,1,1") "Undefined" 0 0))
    (:3
      (Game|SpawnActorfromClass "/Game/SHMUP_starter/Blueprints/LevelStuff/SampleLevel/BP_LevelTest_BottomPart2.BP_LevelTest_BottomPart2_C" (Math|Transform|MakeTransform "0,3500.000000,-600.000000" "0, 0, 0" "1,1,1") "Undefined" 0 0))))

(event Custom|SpawnEnemy
  (params (Type :type Enum_EnemySpawnType%20Enum :default "NewEnumerator0"))
  ;[1 1 1] Spawning
  ;;[1 1 1] Spawn enemy based on type
  (switch Utilities|FlowControl|Switch|SwitchonEnum_EnemySpawnType Type
    (:NewEnumerator0
      (|Regular))
    (:NewEnumerator1
      (|RegularWave))
    (:NewEnumerator2
      (|RegularShooter))
    (:NewEnumerator3
      (|RegularShooterWave))
    (:NewEnumerator4
      (|Asteroid))
    (:NewEnumerator5
      (|AsteroidWave))
    (:NewEnumerator6
      (|Robot))))

(event Custom|PhaseUp
  ;[1 1 1] Level composition (Robots are set to phase up on death.  Basically mini-boss.)
  (Variables|Default|SetDone false)
  (bind _output_get (Variables|Default|SetPhase (+ (Variables|Default|GetPhase) 1)))
  (switch int _output_get
    (:1
      (CallFunction|SpawnDropShip "NewEnumerator7")
      (Utilities|FlowControl|Delay 6.0)
      (CallFunction|SpawnEnemy "NewEnumerator1")
      (Utilities|FlowControl|Delay 2e+01)
      (Variables|Default|SetDone true)
      (Utilities|FlowControl|Delay 5.0)
      (CallFunction|PhaseUp))
    (:2
      (CallFunction|SpawnEnemy "NewEnumerator3")
      (Utilities|FlowControl|Delay 15.0)
      (CallFunction|SpawnDropShip "NewEnumerator8")
      (Utilities|FlowControl|Delay 2e+01)
      (Variables|Default|SetDone true)
      (Utilities|FlowControl|Delay 5.0)
      (CallFunction|PhaseUp))
    (:3
      (CallFunction|SpawnLevelObject 3)
      (Utilities|FlowControl|Delay 25.0)
      (Variables|Default|SetDone true)
      (CallFunction|SpawnDropShip "NewEnumerator7")
      (Utilities|FlowControl|Delay 15.0)
      (CallFunction|PhaseUp))
    (:4
      (CallFunction|SpawnLevelObject 1)
      (CallFunction|SpawnDropShip "NewEnumerator3")
      (Utilities|FlowControl|Delay 22.0)
      (Variables|/Game/SHMUP_starter/Blueprints/Ship/BP_Hero.BP_Hero_C|SetLevelMod1 (Variables|Default|GetHero) true))))

(event Custom|SpawnDropShip
  (params (Drop :type Enum_PickUpType%20Enum :default "NewEnumerator0"))
  ;[1 1 1] Spawning
  ;;[1 1 1] Spawn Drop ship
  (Game|SpawnActorfromClass "/Game/SHMUP_starter/Blueprints/Enemies/BP_EnemyShip_DropShip.BP_EnemyShip_DropShip_C" (Math|Transform|MakeTransform "0,2000.000000,0.000000" "0, 0, 0" "1,1,1") "Undefined" 0 1.0 true Drop 2.5 0.0 false false 2.0 35 0))

(event Custom|StartPhase
  ;[1 1 1] Level composition (Robots are set to phase up on death.  Basically mini-boss.)
  (CallFunction|SpawnEnemy "NewEnumerator1")
  (Utilities|FlowControl|Delay 2e+01)
  (CallFunction|SpawnDropShip "NewEnumerator3")
  (CallFunction|SpawnLevelObject 2)
  (Utilities|FlowControl|Delay 1e+01)
  (CallFunction|SpawnDropShip "NewEnumerator3")
  (Variables|Default|SetDone true)
  (Utilities|FlowControl|Delay 2.0)
  (Variables|Default|SetDone false)
  (CallFunction|SpawnEnemy "NewEnumerator5")
  (Utilities|FlowControl|Delay 2e+01)
  (Variables|Default|SetDone true)
  (Utilities|FlowControl|Delay 1e+01)
  (CallFunction|SpawnEnemy "NewEnumerator6"))

(event EventBeginPlay
  ;[1 1 1] Initialize
  (bind _asbp_hero (Utilities|Casting|CastToBP_Hero (Game|Player|GetPlayerPawn 0)))
  (bind _output_get (Variables|Default|SetHero _asbp_hero))
  (Variables|/Game/SHMUP_starter/Blueprints/Ship/BP_Hero.BP_Hero_C|SetLevelManager _output_get self)
  (Utilities|FlowControl|Delay 1e+01)
  (CallFunction|StartPhase))

(fn ConstructionScript)